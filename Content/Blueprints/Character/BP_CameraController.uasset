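; Player controller that drives a top-down strategy camera over the BP_MapManager map, with cursor visible.
; Each tick MoveCamera combines pan keys with screen-edge scrolling, clamps the pawn to map-derived bounds and lets zoom set speed, pitch and spring arm length, without delta-time scaling.
; Select advances the map's round and recomputes those bounds with a debug box.
; Tile picking and tower creation code is unconnected or never called.
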(event Input|EnhancedActionEvents|EnhancedInputActionIA_Pan_Down
  (params (ActionValue :type Boolean) (ElapsedSeconds :type Float%20%28double-precision%29) (TriggeredSeconds :type Float%20%28double-precision%29) (InputAction :type Input%20Action%20Object%20Reference :default "/Game/Blueprints/Input/IA_Pan_Down.IA_Pan_Down"))
  ;[1 1 1] Inputs
  (:Started
    (Variables|Default|SetCamera%20Movement (+ (Variables|Default|GetCamera%20Movement) "0.000000,1.000000,0.000000")))
  (:Completed
    (Variables|Default|SetCamera%20Movement (- (Variables|Default|GetCamera%20Movement) "0.000000,1.000000,0.000000"))))

(event Input|EnhancedActionEvents|EnhancedInputActionIA_Pan_Left
  (params (ActionValue :type Boolean) (ElapsedSeconds :type Float%20%28double-precision%29) (TriggeredSeconds :type Float%20%28double-precision%29) (InputAction :type Input%20Action%20Object%20Reference :default "/Game/Blueprints/Input/IA_Pan_Left.IA_Pan_Left"))
  ;[1 1 1] Inputs
  (:Started
    (Variables|Default|SetCamera%20Movement (+ (Variables|Default|GetCamera%20Movement) "-1.000000,0.000000,0.000000")))
  (:Completed
    (Variables|Default|SetCamera%20Movement (- (Variables|Default|GetCamera%20Movement) "-1.000000,0.000000,0.000000"))))

(event Input|EnhancedActionEvents|EnhancedInputActionIA_Pan_Up
  (params (ActionValue :type Boolean) (ElapsedSeconds :type Float%20%28double-precision%29) (TriggeredSeconds :type Float%20%28double-precision%29) (InputAction :type Input%20Action%20Object%20Reference :default "/Game/Blueprints/Input/IA_Pan_Up.IA_Pan_Up"))
  ;[1 1 1] Inputs
  (:Started
    (Variables|Default|SetCamera%20Movement (+ (Variables|Default|GetCamera%20Movement) "0.000000,-1.000000,0.000000")))
  (:Completed
    (Variables|Default|SetCamera%20Movement (- (Variables|Default|GetCamera%20Movement) "0.000000,-1.000000,0.000000"))))

(event Input|EnhancedActionEvents|EnhancedInputActionIA_Pan_Right
  (params (ActionValue :type Boolean) (ElapsedSeconds :type Float%20%28double-precision%29) (TriggeredSeconds :type Float%20%28double-precision%29) (InputAction :type Input%20Action%20Object%20Reference :default "/Game/Blueprints/Input/IA_Pan_Right.IA_Pan_Right"))
  ;[1 1 1] Inputs
  (:Started
    (Variables|Default|SetCamera%20Movement (+ (Variables|Default|GetCamera%20Movement) "1.000000,0.000000,0.000000")))
  (:Completed
    (Variables|Default|SetCamera%20Movement (- (Variables|Default|GetCamera%20Movement) "1.000000,0.000000,0.000000"))))

(event Input|EnhancedActionEvents|EnhancedInputActionIA_Zoom
  (params (ActionValue :type Vector%202D%20Structure) (ElapsedSeconds :type Float%20%28double-precision%29) (TriggeredSeconds :type Float%20%28double-precision%29) (InputAction :type Input%20Action%20Object%20Reference :default "/Game/Blueprints/Input/IA_Zoom.IA_Zoom"))
  ;[1 1 1] Inputs
  (Variables|Default|SetCamera%20Zoom (Math|Float|Clamp(Float) (+ (* (.x ActionValue) -0.1) (Variables|Default|GetCamera%20Zoom)))))

(event Input|EnhancedActionEvents|EnhancedInputActionIA_Select
  (params (ActionValue :type Boolean) (ElapsedSeconds :type Float%20%28double-precision%29) (TriggeredSeconds :type Float%20%28double-precision%29) (InputAction :type Input%20Action%20Object%20Reference :default "/Game/Blueprints/Input/IA_Select.IA_Select"))
  (Default|IncrementRound (Variables|Default|GetMap))
  (CallFunction|RedrawCameraBounds))

(event EventBeginPlay
  (bind _returnvalue (PlayerController|LocalPlayerSubsystems|GetEnhancedInputLocalPlayerSubsystem))
  (Variables|Default|SetbShowMouseCursor true)
  (Utilities|IsValid _returnvalue
    (:Is%20Valid
      (Input|AddMappingContext _returnvalue "/Game/Blueprints/Input/IMC_CameraInput.IMC_CameraInput" 0 "(bIgnoreAllPressedKeysUntilRelease=True,bForceImmediately=False,bNotifyUserSettings=False)")
      (Variables|Default|SetCamera%20Pawn (Game|Player|GetPlayerPawn 0))
      (bind _returnvalue_2 (Actor|GetActorOfClass "/Game/Blueprints/Map/BP_MapManager.BP_MapManager_C"))
      (Variables|Default|SetMap _returnvalue_2)
      (CallFunction|RedrawCameraBounds)
      (Input|SetInputModeGameandUI self 0 "LockOnCapture" true false))))

(event EventTick
  (params (DeltaSeconds :type Float%20%28single-precision%29))
  (CallFunction|MoveCamera))

(fn ConstructionScript)

(fn MoveCamera
  (bind _returnvalue (Viewport|GetViewportSize))
  (bind _returnvalue_2 (Viewport|GetViewportSize))
  (bind _camera_pawn (Variables|Default|GetCamera%20Pawn))
  (bind _grid_size_x (Variables|Default|GetGrid%20Size%20X))
  (bind _grid_size_y (Variables|Default|GetGrid%20Size%20Y))
  (bind _returnvalue_3 (Class|WidgetLayoutLibrary|GetMousePositiononViewport))
  (LocalVariables|SetMouse%20X (.x _returnvalue_3))
  (LocalVariables|SetMouse%20Y (.y _returnvalue_3))
  (Transformation|SetActorLocationAndRotation _camera_pawn (Math|Vector|MakeVector (Math|Float|Clamp(Float) (.x (+ (Transformation|GetActorLocation _camera_pawn) (* (Math|Vector|Normalize (Utilities|Operators|Subtract (Math|Vector|Normalize (Variables|Default|GetCamera%20Movement)) (Math|Vector|MakeVector (- 1.0 (Math|Float|Clamp(Float) (Math|Float|NormalizetoRange (LocalVariables|GetMouse%20X) 0.0 (* (.x (Viewport|GetViewportSize)) 0.05)))) 0.0 0.0) (Math|Vector|MakeVector (* (Math|Float|Clamp(Float) (Math|Float|NormalizetoRange (LocalVariables|GetMouse%20X) (* (.x _returnvalue_2) 0.95) (.x _returnvalue_2))) -1.0) 0.0 0.0) (Math|Vector|MakeVector 0.0 (- 1.0 (Math|Float|Clamp(Float) (Math|Float|NormalizetoRange (LocalVariables|GetMouse%20Y) 0.0 (* (.y (Viewport|GetViewportSize)) 0.05)))) 0.0) (Math|Vector|MakeVector 0.0 (* (Math|Float|Clamp(Float) (Math|Float|NormalizetoRange (LocalVariables|GetMouse%20Y) (* (.y _returnvalue) 0.95) (.y _returnvalue))) -1.0) 0.0))) (Math|Float|Lerp (Variables|Default|GetMinimum%20Camera%20Speed) (Variables|Default|GetMaximum%20Camera%20Speed) (Variables|Default|GetCamera%20Zoom))))) (* _grid_size_x -1.0) _grid_size_x) (Math|Float|Clamp(Float) (.y (+ (Transformation|GetActorLocation _camera_pawn) (* (Math|Vector|Normalize (Utilities|Operators|Subtract (Math|Vector|Normalize (Variables|Default|GetCamera%20Movement)) (Math|Vector|MakeVector (- 1.0 (Math|Float|Clamp(Float) (Math|Float|NormalizetoRange (LocalVariables|GetMouse%20X) 0.0 (* (.x (Viewport|GetViewportSize)) 0.05)))) 0.0 0.0) (Math|Vector|MakeVector (* (Math|Float|Clamp(Float) (Math|Float|NormalizetoRange (LocalVariables|GetMouse%20X) (* (.x _returnvalue_2) 0.95) (.x _returnvalue_2))) -1.0) 0.0 0.0) (Math|Vector|MakeVector 0.0 (- 1.0 (Math|Float|Clamp(Float) (Math|Float|NormalizetoRange (LocalVariables|GetMouse%20Y) 0.0 (* (.y (Viewport|GetViewportSize)) 0.05)))) 0.0) (Math|Vector|MakeVector 0.0 (* (Math|Float|Clamp(Float) (Math|Float|NormalizetoRange (LocalVariables|GetMouse%20Y) (* (.y _returnvalue) 0.95) (.y _returnvalue))) -1.0) 0.0))) (Math|Float|Lerp (Variables|Default|GetMinimum%20Camera%20Speed) (Variables|Default|GetMaximum%20Camera%20Speed) (Variables|Default|GetCamera%20Zoom))))) (* _grid_size_y -1.0) _grid_size_y) 2.5e+02) (Math|Rotator|MakeRotator 0.0 (Math|Float|Lerp 15.0 0.0 (Variables|Default|GetCamera%20Zoom)) -9e+01))
  (bind _asbp_camera_pawn (Utilities|Casting|CastToBP_CameraPawn (Variables|Default|GetCamera%20Pawn)))
  (Variables|/Script/Engine.SpringArmComponent|SetTargetArmLength (Variables|/Game/Blueprints/Character/BP_CameraPawn.BP_CameraPawn_C|GetSpringArm _asbp_camera_pawn) (Math|Float|Lerp (Variables|Default|GetMinimum%20Camera%20Zoom) (Variables|Default|GetMaximum%20Camera%20Zoom) (Variables|Default|GetCamera%20Zoom))))

(fn ConvertWorldCoordtoChunkCoord
  (bind _output_get (LocalVariables|SetHitActor (.hitactor (.HitResult (Game|Player|GetHitResultUnderCursorbyChannel "TraceTypeQuery1" true)))))
  (bind _asbp_tile (Utilities|Casting|CastToBP_Tile _output_get))
  (Development|PrintText "Selected the Tile!")
  (Development|PrintText (Utilities|Text|FormatText "Hit Entity at position ({X},{Y},{Z})" (.x (.location (Transformation|GetWorldTransform (Transformation|GetAttachParent (Variables|/Game/Blueprints/Map/BP_Tile.BP_Tile_C|GetDefaultSceneRoot _asbp_tile))))) (.y (.location (Transformation|GetWorldTransform (Transformation|GetAttachParent (Variables|/Game/Blueprints/Map/BP_Tile.BP_Tile_C|GetDefaultSceneRoot _asbp_tile))))) (.z (.location (Transformation|GetWorldTransform (Transformation|GetAttachParent (Variables|/Game/Blueprints/Map/BP_Tile.BP_Tile_C|GetDefaultSceneRoot _asbp_tile))))))))

(fn RedrawCameraBounds
  (bind _map (Variables|Default|GetMap))
  (bind (_origin _boxextent) (Collision|GetActorBounds _map false true))
  (bind _output_get (Variables|Default|SetGrid%20Size%20X (* (.x _boxextent) 2.0)))
  (bind _output_get_2 (Variables|Default|SetGrid%20Size%20Y (* (.y _boxextent) 2.0)))
  (Rendering|Debug|DrawDebugBox _origin (Math|Vector|MakeVector _output_get _output_get_2 5e+02) "(R=1.000000,G=0.000000,B=0.315240,A=1.000000)" "0, 0, 0" 2e+01 0.0))