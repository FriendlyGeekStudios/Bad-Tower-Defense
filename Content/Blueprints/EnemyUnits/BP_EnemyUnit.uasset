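; Enemy unit character that targets the map's tagged Headquarter, with stats, mesh, animation and attack montage configured from a spawn card.
; BeginPlay writes the headquarters position to the AI blackboard, and Tick updates an in-range flag from the distance band.
; AttackTower plays the montage unless already playing, while a separate EmitDamage event damages the headquarters.
; Incoming damage lowers health and refreshes the health bar widget, with no death handling here.
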(event Custom|Event%20Attack%20Tower
  (if (not (Animation|Montage|MontageIsPlaying (Components|SkeletalMesh|GetAnimInstance (Variables|Character|GetMesh)) (Variables|Default|GetAttack%20Animation%20Montage)))
    (Animation|PlayAnimMontage (Variables|Default|GetAttack%20Animation%20Montage) 1.0 "None")))

(event Custom|Event%20Emit%20Damage
  (Game|Damage|ApplyDamage (Variables|Default|GetHeadquarter) (Variables|Default|GetAttack%20Damage) 0 0))

(event EventBeginPlay
  (CallFunction|UpdateHealthBar)
  (bind _outactors (Actor|GetAllActorswithTag "Headquarter"))
  (if (Utilities|Array|IsEmpty _outactors)
    (Development|PrintText "Could not find headquarters in map")
    (else
      (bind _output_get (Variables|Default|SetHeadquarter (Utilities|Array|Get(acopy) _outactors)))
      (bind _output_get_2 (Variables|Default|SetTarget%20Location (Transformation|GetActorLocation _output_get)))
      (AI|Components|Blackboard|SetValueasVector (AI|GetBlackboard (AI|GetAIController self)) (Utilities|Name|MakeLiteralName "Target Position") (Math|Vector|MakeVector (.x _output_get_2) (.y _output_get_2) (.z (Transformation|GetActorLocation)))))))

(event EventTick
  (params (DeltaSeconds :type Float%20%28single-precision%29))
  (bind _returnvalue (Transformation|GetActorLocation))
  (bind _target_location (Variables|Default|GetTarget%20Location))
  (bind _returnvalue_2 (- _returnvalue _target_location))
  (bind _returnvalue_3 (Math|Vector|VectorLength _returnvalue_2))
  (AI|Components|Blackboard|SetValueasBool (AI|GetBlackboard (AI|GetAIController self)) (Utilities|Name|MakeLiteralName "bIsInRange") (and (< _returnvalue_3 (Variables|Default|GetMaximum%20Range)) (> _returnvalue_3 (Variables|Default|GetMinimum%20Range)))))

(event Game|Damage|EventAnyDamage
  (params (Damage :type Float%20%28single-precision%29) (DamageType :type Damage%20Type%20Object%20Reference) (InstigatedBy :type Controller%20Object%20Reference) (DamageCauser :type Actor%20Object%20Reference))
  (Variables|Default|SetCurrent%20Heatlh (- (Variables|Default|GetCurrent%20Heatlh) Damage))
  (CallFunction|UpdateHealthBar))

(fn ConstructionScript)

(fn ConfigureEnemyUnit
  (params (Spawn%20Card :type BPS%20Enemy%20Unit%20Stats%20Base%20Structure))
  (bind (_charactername _basehealth _movementspeed _attackspeed _attackdamage _spawncost _spawnweight _roundrequirement _experiencereward _currencyreward _characterskeleton _characteranimation _minimumrange _maximumrange _attackanimationmontage) (Utilities|Struct|BreakBPS_EnemyUnit_StatsBase Spawn%20Card))
  (Variables|Default|SetName _charactername)
  (bind _output_get (Variables|Default|SetMax%20Health _basehealth))
  (Variables|Default|SetCurrent%20Heatlh _output_get)
  (CallFunction|UpdateHealthBar)
  (Variables|Default|SetMovement%20Speed _movementspeed)
  (Variables|Default|SetAttack%20Speed _attackspeed)
  (Variables|Default|SetAttack%20Damage _attackdamage)
  (Variables|Default|SetExperience%20Reward _experiencereward)
  (Variables|Default|SetCurrency%20Reward _currencyreward)
  (Components|SkeletalMesh|SetSkeletalMeshAsset (Variables|Character|GetMesh) _characterskeleton)
  (Class|SkeletalMeshComponent|SetAnimClass (Variables|Character|GetMesh) _characteranimation)
  (Variables|Default|SetMinimum%20Range _minimumrange)
  (Variables|Default|SetMaximum%20Range _maximumrange)
  (Variables|Default|SetAttack%20Animation%20Montage _attackanimationmontage))

(fn UpdateHealthBar
  (bind _ashealth_bar (Utilities|Casting|CastToHealthBar (UserInterface|GetUserWidgetObject (Variables|Default|GetHealthBar))))
  (Variables|/Game/Blueprints/UI/HealthBar.HealthBar_C|SetHealth _ashealth_bar (Math|Conversions|ToFloat(Integer) (/ (Variables|Default|GetCurrent%20Heatlh) (Variables|Default|GetMax%20Health)))))