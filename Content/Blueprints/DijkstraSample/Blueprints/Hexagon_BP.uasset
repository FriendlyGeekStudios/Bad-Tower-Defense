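; Hexagon_BP is a clickable hexagon cell in a grid for a Dijkstra pathfinding sample.
; SetUpCell styles the cell from its flags, stretching obstacles vertically and toggling the Resource and End markers' visibility, with materials reapplied to each.
; Clicking the mesh of a non-obstacle cell forwards it to the parent grid through CellClicked.
; The construction script applies a material to the mesh.
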(event OnClicked(StaticMeshComponent)
  (params (TouchedComponent :type Primitive%20Component%20Object%20Reference) (ButtonPressed :type Key%20Structure))
  ;[1 1 1] Propagate the click to the parent grid
  (if (not (Variables|Default|GetIsObstacle))
    (CallFunction|CellClicked (.ParentGrid (Variables|Default|GetParentGrid)) self)))

(event Custom|SetUpCell
  ;[1 1 1] Change properties if it is an obstacle
  (if (Variables|Default|GetIsObstacle)
    (Transformation|SetActorScale3D "1.000000,1.000000,5.000000")
    (Rendering|Material|SetMaterial (Variables|Debug|GetStaticMeshComponent) 0 0)
    (else
      (Transformation|SetActorScale3D "1.000000,1.000000,1.000000")
      (Rendering|Material|SetMaterial (Variables|Debug|GetStaticMeshComponent) 0 0)))
  (Rendering|SetVisibility (Variables|Default|GetResource) (Variables|Default|GetIsResource) false)
  (Rendering|Material|SetMaterial (Variables|Default|GetResource) 0 0)
  (Rendering|SetVisibility (Variables|Default|GetEnd) (Variables|Default|GetIsEnd) false)
  (Rendering|Material|SetMaterial (Variables|Default|GetEnd) 0 0))

(fn ConstructionScript
  (Rendering|Material|SetMaterial (Variables|Debug|GetStaticMeshComponent) 0 0)
  (Utilities|FlowControl|Sequence))