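; BP_Chunk is one square chunk of the map that builds a hex tile grid and carves a random road across it.
; Generate spawns BP_Tile child actors in offset rows and labels the chunk with its coordinate.
; GeneratePath picks an exit edge facing the next chunk, converts DijkstraRandomPath results to road and debug-colors both endpoints.
; Randomness comes from the map manager's shared utility or BP_RandomWrapper; a local Dijkstra also exists but GeneratePath bypasses it.
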(event EventBeginPlay)

(event Collision|EventActorBeginOverlap
  (params (OtherActor :type Actor%20Object%20Reference)))

(event EventTick
  (params (DeltaSeconds :type Float%20%28single-precision%29)))

(fn ConstructionScript
  (bind _asbp_map_manager (Utilities|Casting|CastToBP_MapManager (Components|GetOwner (Variables|Default|GetDefaultSceneRoot)))
    (:then
      (Variables|Default|SetRandom%20Noise%20Util (Variables|/Game/Blueprints/Map/BP_MapManager.BP_MapManager_C|GetRandom%20Noise%20Util _asbp_map_manager)))
    (:CastFailed
      (bind _returnvalue (Actor|GetActorOfClass "/Game/Blueprints/BP_RandomWrapper.BP_RandomWrapper_C"))
      (Variables|Default|SetRandom%20Noise%20Util _returnvalue))))

(fn Generate
  (params (New%20Chunk%20Size :type Integer) (Coordinate%20X :type Integer) (Coordinate%20Y :type Integer))
  (|ConfigureParameters New%20Chunk%20Size Coordinate%20X Coordinate%20Y (.x (.max (StaticMesh|GetBoundingBox (Variables|GridOptions|GetTile%20Mesh)))))
  (for _index (range 0 (- (Variables|GridOptions|GetChunkWidth) 1))
    (for _index_2 (range 0 (- (Variables|GridOptions|GetChunkHeight) 1))
      (bind _returnvalue (AddComponent|AddChildActorComponent false (Math|Transform|MakeTransform (Math|Vector|MakeVector (.x (Math|Vector|SelectVector (Math|Vector|MakeVector (* (Variables|GridOptions|GetRadius) _index 2.0) (* _index_2 1.5 (/ (* (Variables|GridOptions|GetRadius) 2.0) (Math|Float|Sqrt 3.0))) 0.0) (Math|Vector|MakeVector (+ (* (Variables|GridOptions|GetRadius) _index 2.0) (Variables|GridOptions|GetRadius)) (* _index_2 1.5 (/ (* (Variables|GridOptions|GetRadius) 2.0) (Math|Float|Sqrt 3.0))) 0.0) (== (Math|Integer|%(Integer) _index_2 2) 0))) (.y (Math|Vector|SelectVector (Math|Vector|MakeVector (* (Variables|GridOptions|GetRadius) _index 2.0) (* _index_2 1.5 (/ (* (Variables|GridOptions|GetRadius) 2.0) (Math|Float|Sqrt 3.0))) 0.0) (Math|Vector|MakeVector (+ (* (Variables|GridOptions|GetRadius) _index 2.0) (Variables|GridOptions|GetRadius)) (* _index_2 1.5 (/ (* (Variables|GridOptions|GetRadius) 2.0) (Math|Float|Sqrt 3.0))) 0.0) (== (Math|Integer|%(Integer) _index_2 2) 0))) 0.0) "0, 0, 0" "1.000000,1.000000,1.000000")))
      (bind _asbp_tile (Utilities|Casting|CastToBP_Tile (Variables|/Script/Engine.ChildActorComponent|GetChildActor _returnvalue)))
      (Utilities|Array|Add (Variables|Default|GetTiles) _asbp_tile)
      (Default|Generate _asbp_tile _index _index_2)))
  (Rendering|Components|TextRender|SetText (Variables|Default|GetChunk%20Label) (Utilities|Text|FormatText "({X}, {Y})" (Variables|Default|GetCoordinate%20X) (Variables|Default|GetCoordinate%20Y)))
  (return self))

(fn SelectRandomLandTile
  (bind _random_noise_util (Variables|Default|GetRandom%20Noise%20Util))
  (bind _tiles (Variables|Default|GetTiles))
  (bind _tiles_2 (Variables|Default|GetTiles))
  (bind _returnvalue (Utilities|Array|LastIndex _tiles))
  (bind _return_value (Default|GetRandomIntegerinRange _random_noise_util 0 _returnvalue))
  (bind _output (Utilities|Array|Get(acopy) _tiles_2 _return_value))
  (while (not (LocalVariables|GetFound%20Tile))
    (LocalVariables|SetFound%20Tile (Utilities|Enum|Equal(Enum) (Variables|/Game/Blueprints/Map/BP_Tile.BP_Tile_C|GetTile%20Type _output) "NewEnumerator2")))
  (return _output))

(fn GeneratePath
  (params (Starting%20Tile%20Coordinate :type Coordinate%202D%20Structure) (Next%20Chunk%20Coordinate :type Coordinate%202D%20Structure))
  (bind _chunkheight (Variables|GridOptions|GetChunkHeight))
  (bind _chunkheight_2 (Variables|GridOptions|GetChunkHeight))
  ;[1 1 1] Select Coordinates for the End Tile
  (bind _output_get (Variables|Default|SetPath%20Start%20Coordinate Starting%20Tile%20Coordinate))
  (if (not (== (Variables|Default|GetCoordinate%20X) (.x Next%20Chunk%20Coordinate)))
    (if (< (.x Next%20Chunk%20Coordinate) (Variables|Default|GetCoordinate%20X))
      (LocalVariables|SetEnd%20X 0)
      (else
        (LocalVariables|SetEnd%20X (- _chunkheight 1))))
    (LocalVariables|SetEnd%20Y (Default|GetRandomIntegerinRange (Variables|Default|GetRandom%20Noise%20Util) 1 (- _chunkheight 2)))
    (else
      (if (< (.y Next%20Chunk%20Coordinate) (Variables|Default|GetCoordinate%20Y))
        (LocalVariables|SetEnd%20Y 0)
        (else
          (LocalVariables|SetEnd%20Y (- _chunkheight_2 1))))
      (LocalVariables|SetEnd%20X (Default|GetRandomIntegerinRange (Variables|Default|GetRandom%20Noise%20Util) 1 (- _chunkheight_2 2)))))
  (bind _output_get_2 (Variables|Default|SetPath%20End%20Coordinate (Utilities|Struct|MakeCoordinate2D (LocalVariables|GetEnd%20X) (LocalVariables|GetEnd%20Y))))
  (Development|PrintText (Utilities|Text|FormatText "Finding Chunk Local Path from ({Start X}, {Start Y}) to ({End X}, {End Y})" (.X (Utilities|Struct|BreakCoordinate2D (Variables|Default|GetPath%20Start%20Coordinate))) (.Y (Utilities|Struct|BreakCoordinate2D (Variables|Default|GetPath%20Start%20Coordinate))) (LocalVariables|GetEnd%20X) (LocalVariables|GetEnd%20Y)))
  (bind _returnvalue (Class|RandomWalkLibrary|DijkstraRandomPath _output_get _output_get_2 (Variables|/Game/Blueprints/BP_RandomWrapper.BP_RandomWrapper_C|GetRandomStream (Variables|Default|GetRandom%20Noise%20Util)) 8))
  (for _array_element _returnvalue
    (bind _returnvalue_2 (Class|MapUtilitiesLibrary|ConvertCoordinatestoIndex (.x _array_element) (.y _array_element) 8))
    (Default|ConverttoRoadTile (Utilities|Array|Get(acopy) (Variables|Default|GetTiles) _returnvalue_2)))
  (bind _returnvalue_3 (Class|MapUtilitiesLibrary|ConvertCoordinatestoIndex (.x (Variables|Default|GetPath%20Start%20Coordinate)) (.y (Variables|Default|GetPath%20Start%20Coordinate)) 8))
  (bind _returnvalue_4 (Rendering|Material|CreateDynamicMaterialInstance "/Game/Materials/M_MaterialDebug.M_MaterialDebug" "None" "None" :!class /Script/Engine.KismetMaterialLibrary))
  (Default|UpdateMaterial (Utilities|Array|Get(acopy) (Variables|Default|GetTiles) _returnvalue_3) _returnvalue_4)
  (bind _returnvalue_5 (Class|MapUtilitiesLibrary|ConvertCoordinatestoIndex (.x (Variables|Default|GetPath%20End%20Coordinate)) (.y (Variables|Default|GetPath%20End%20Coordinate)) 8))
  (bind _returnvalue_6 (Rendering|Material|CreateDynamicMaterialInstance "/Game/Materials/M_MaterialDebug.M_MaterialDebug" "None" "None" :!class /Script/Engine.KismetMaterialLibrary))
  (Rendering|Material|SetVectorParameterValue _returnvalue_6 "Color" "(R=0.000000,G=0.407807,B=1.000000,A=1.000000)" :!class /Script/Engine.MaterialInstanceDynamic)
  (Default|UpdateMaterial (Utilities|Array|Get(acopy) (Variables|Default|GetTiles) _returnvalue_5) _returnvalue_6))

(fn DebugTiles
  (for _array_element (Variables|Default|GetTiles)
    (bind _returnvalue (Class|MapUtilitiesLibrary|IsNonCornerEdgeTile (Variables|/Game/Blueprints/Map/BP_Tile.BP_Tile_C|GetCoordinate%20X _array_element) (Variables|/Game/Blueprints/Map/BP_Tile.BP_Tile_C|GetCoordinate%20Y _array_element) (Variables|GridOptions|GetChunkWidth)))
    (if _returnvalue
      (Rendering|Material|SetMaterial (Variables|/Game/Blueprints/Map/BP_Tile.BP_Tile_C|GetTile _array_element) 0 "/Game/Materials/M_Road.M_Road"))))

(fn GetGlobalTileCoordinate
  (params (Chunk%20Local%20Tile%20Coordinate :type Coordinate%202D%20Structure))
  (return (Utilities|Struct|MakeCoordinate2D (+ (.x Chunk%20Local%20Tile%20Coordinate) (Variables|Default|GetCoordinate%20X)) (+ (.y Chunk%20Local%20Tile%20Coordinate) (Variables|Default|GetCoordinate%20Y)))))

(fn GetChunkLocalCoordinatefromGlobalCoordinate
  (params (Global%20Coordinate :type Coordinate%202D%20Structure))
  (return (Utilities|Struct|MakeCoordinate2D (Math|Integer|%(Integer) (.x Global%20Coordinate) (Variables|GridOptions|GetChunkWidth)) (Math|Integer|%(Integer) (.y Global%20Coordinate) (Variables|GridOptions|GetChunkWidth)))))

(fn Dijkstra
  (params (Start :type Coordinate%202D%20Structure) (End :type Coordinate%202D%20Structure))
  (bind _results (LocalVariables|GetResults))
  (bind _chunkwidth (Variables|GridOptions|GetChunkWidth))
  (bind _returnvalue (- _chunkwidth 1))
  (LocalVariables|SetStart%20Coordinate Start)
  (bind _output_get (LocalVariables|SetEnd%20Coordinate End))
  (Utilities|FlowControl|Sequence
    (:then_0
      (LocalVariables|SetFrontier (Utilities|Array|MakeArray (LocalVariables|GetStart%20Coordinate)))
      (LocalVariables|SetCame%20From (Utilities|Map|MakeMap (LocalVariables|GetStart%20Coordinate) ""))
      (LocalVariables|SetCost%20So%20Far (Utilities|Map|MakeMap (LocalVariables|GetStart%20Coordinate) 0)))
    (:then_1
      (if (Utilities|Array|IsNotEmpty (LocalVariables|GetFrontier))
        (while (and (Utilities|Array|IsNotEmpty (LocalVariables|GetFrontier)) (not (Utilities|CompareCoordinates _output_get (Utilities|Array|Get(acopy) (LocalVariables|GetFrontier)))))
          (bind _output_get_2 (LocalVariables|SetCurrent (Utilities|Array|Get(acopy) (LocalVariables|GetFrontier))))
          (Utilities|Array|RemoveIndex (LocalVariables|GetFrontier))
          (for _array_element (Class|RandomWalkLibrary|GetAllNeighbors _output_get_2 (Variables|GridOptions|GetChunkHeight))
            (if (or (Utilities|CompareCoordinates (LocalVariables|GetEnd%20Coordinate) _array_element) (Math|Boolean|ANDBoolean (> (.X (Utilities|Struct|BreakCoordinate2D _array_element)) 0) (< (.X (Utilities|Struct|BreakCoordinate2D _array_element)) _returnvalue) (> (.Y (Utilities|Struct|BreakCoordinate2D _array_element)) 0) (< (.Y (Utilities|Struct|BreakCoordinate2D _array_element)) _returnvalue)))
              (bind _output_get_3 (LocalVariables|SetNew%20Cost (+ (.Value (Utilities|Map|Find (LocalVariables|GetCost%20So%20Far) (LocalVariables|GetCurrent))) (Default|GetRandomIntegerinRange (Variables|Default|GetRandom%20Noise%20Util)))))
              (if (or (and (< _output_get_3 (.Value (Utilities|Map|Find (LocalVariables|GetCost%20So%20Far) _array_element))) (.ReturnValue (Utilities|Map|Find (LocalVariables|GetCost%20So%20Far) _array_element))) (not (Utilities|Map|Contains (LocalVariables|GetCost%20So%20Far) _array_element)))
                (Utilities|Map|Add (LocalVariables|GetCost%20So%20Far) _array_element _output_get_3)
                (Utilities|Array|Add (LocalVariables|GetFrontier) _array_element)
                (Utilities|Map|Add (LocalVariables|GetCame%20From) _array_element (LocalVariables|GetCurrent))))))
        ;[1 1 1] Backtrack...
        (LocalVariables|SetCurrent (LocalVariables|GetEnd%20Coordinate))
        (while (not (Utilities|CompareCoordinates (LocalVariables|GetStart%20Coordinate) (LocalVariables|GetCurrent)))
          (Utilities|Array|Add (LocalVariables|GetResults) (LocalVariables|GetCurrent))
          (LocalVariables|SetCurrent (.Value (Utilities|Map|Find (LocalVariables|GetCame%20From) (LocalVariables|GetCurrent)))))
        (Development|PrintText (Utilities|Text|FormatText "Selected Tiles for chunk ({X}, {Y}) (Reversed)" (Variables|Default|GetCoordinate%20X) (Variables|Default|GetCoordinate%20Y)))
        (Utilities|Array|Add (LocalVariables|GetResults) (LocalVariables|GetStart%20Coordinate))
        (for _array_element_2 _results
          (Development|PrintText (Utilities|Text|FormatText "Path Includes Chunk Coordinate ({X}, {Y}) [G:({Global X},{Global Y})]" (.x _array_element_2) (.y _array_element_2) (.x (CallFunction|GetGlobalTileCoordinate (Utilities|Struct|MakeCoordinate2D (.x _array_element_2) (.y _array_element_2)))) (.y (CallFunction|GetGlobalTileCoordinate (Utilities|Struct|MakeCoordinate2D (.x _array_element_2) (.y _array_element_2)))))))
        (return _results)))))