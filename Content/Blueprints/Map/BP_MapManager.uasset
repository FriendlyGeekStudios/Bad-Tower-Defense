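; Map manager for a tower defense game that grows a tiled world chunk by chunk as rounds advance.
; Construction uses the seeded BP_RandomWrapper stream in DimerizationWalk to order chunk coordinates, then spawns BP_Chunk child actors up to CurrentRound, spaced by tile mesh bounds.
; IncrementRound adds the next chunk and generates its path toward the following one.
; BeginPlay builds the headquarters on HeadquarterTile, but the construction calls selecting that tile and pathing the chunk are disconnected.
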(event EventBeginPlay
  (CallFunction|SpawnDefenseHeadquarters))

(event Collision|EventActorBeginOverlap
  (params (OtherActor :type Actor%20Object%20Reference)))

(event EventTick
  (params (DeltaSeconds :type Float%20%28single-precision%29)))

(fn ConstructionScript
  (bind _tilemesh (Variables|WorldSettings|GetTileMesh))
  (bind _returnvalue (StaticMesh|GetBoundingBox _tilemesh))
  (bind _returnvalue_2 (Actor|GetActorOfClass "/Game/Blueprints/BP_RandomWrapper.BP_RandomWrapper_C"))
  (Utilities|IsValid _returnvalue_2
    (:Is%20Valid
      (Variables|Default|SetRandom%20Noise%20Util _returnvalue_2)
      (Variables|WorldSettings|SetTile%20Radius (.x (.max _returnvalue)))
      (Variables|WorldSettings|SetTile%20Outer%20Radius (.y (.max _returnvalue)))
      (bind _returnvalue_3 (Class|RandomWalkLibrary|DimerizationWalk (Variables|WorldSettings|GetWorld%20Map%20Size%20%28Tiles%29) (Variables|/Game/Blueprints/BP_RandomWrapper.BP_RandomWrapper_C|GetRandomStream (Variables|Default|GetRandom%20Noise%20Util))))
      (Variables|Default|SetAll%20Tile%20Coordinates _returnvalue_3)
      (for _index (range 0 (Variables|Default|GetCurrent%20Round))
        (CallFunction|SpawnNewChunk (.x (Utilities|Array|Get(acopy) (Variables|Default|GetAll%20Tile%20Coordinates) _index)) (.y (Utilities|Array|Get(acopy) (Variables|Default|GetAll%20Tile%20Coordinates) _index))))
      (Development|PrintText "Completed Chunk Generation"))
    (:Is%20Not%20Valid
      (Development|PrintText "Failed to find Random Wrapper"))))

(fn SpawnNewChunk
  (params (Chunk%20Position%20X :type Integer) (Chunk%20Position%20Y :type Integer))
  (bind _returnvalue (AddComponent|AddChildActorComponent false (Math|Transform|MakeTransform (Math|Vector|MakeVector (* Chunk%20Position%20X (* (Variables|WorldSettings|GetTile%20Radius) 2.0) (Variables|WorldSettings|GetChunk%20Size)) (* Chunk%20Position%20Y (* (Variables|WorldSettings|GetTile%20Outer%20Radius) 1.5) (Variables|WorldSettings|GetChunk%20Size)) 0.0) "0, 0, 0" "1.000000,1.000000,1.000000")))
  (bind _asbp_chunk (Utilities|Casting|CastToBP_Chunk (Variables|/Script/Engine.ChildActorComponent|GetChildActor _returnvalue))
    (:then
      (Utilities|Array|Add (Variables|Default|GetChunks) _asbp_chunk)
      (Default|Generate _asbp_chunk (Variables|WorldSettings|GetChunk%20Size) Chunk%20Position%20X Chunk%20Position%20Y)
      (return 0))
    (:CastFailed
      (Development|PrintText "Failed to create new Chunk"))))

(fn GetChunkDimensions
  (bind _chunk_size (Variables|WorldSettings|GetChunk%20Size))
  (return (Math|Vector2D|MakeVector2D (* (Variables|WorldSettings|GetTile%20Radius) 2.0 _chunk_size) (* _chunk_size 1.5 (Variables|WorldSettings|GetTile%20Outer%20Radius)))))

(fn SpawnDefenseHeadquarters
  (Default|CreateTower (Variables|Default|GetHeadquarter%20Tile) "/Game/Blueprints/Towers/BP_Tower_Headquarter.BP_Tower_Headquarter_C"))

(fn SpawnRoadRoute)

(fn FindHeadquarterTile
  (bind _chunk_size (Variables|WorldSettings|GetChunk%20Size))
  (bind _random_noise_util (Variables|Default|GetRandom%20Noise%20Util))
  (bind _returnvalue (- _chunk_size 2))
  (bind _returnvalue_2 (Class|MapUtilitiesLibrary|ConvertCoordinatestoIndex (Default|GetRandomIntegerinRange _random_noise_util 2 _returnvalue) (Default|GetRandomIntegerinRange _random_noise_util 2 _returnvalue) (Variables|WorldSettings|GetChunk%20Size)))
  (bind _output_get (Variables|Default|SetHeadquarter%20Tile (Utilities|Array|Get(acopy) (Variables|/Game/Blueprints/Map/BP_Chunk.BP_Chunk_C|GetTiles (Utilities|Array|Get(acopy) (Variables|Default|GetChunks))) _returnvalue_2)))
  (Rendering|Material|SetOverlayMaterial (Variables|/Game/Blueprints/Map/BP_Tile.BP_Tile_C|GetTile _output_get) "/Game/Materials/M_Highlight.M_Highlight" :!class /Script/Engine.MeshComponent))

(fn IncrementRound
  (bind _all_tile_coordinates (Variables|Default|GetAll%20Tile%20Coordinates))
  (bind _result (Math|Integer|IncrementInt (Variables|Default|GetCurrent%20Round))
    (:%20%20
      (if (< _result (Utilities|Array|Length (Variables|Default|GetAll%20Tile%20Coordinates)))
        (bind _new_chunk (CallFunction|SpawnNewChunk (.x (Utilities|Array|Get(acopy) (Variables|Default|GetAll%20Tile%20Coordinates) _result)) (.y (Utilities|Array|Get(acopy) (Variables|Default|GetAll%20Tile%20Coordinates) _result))))
        (Default|GeneratePath _new_chunk (Utilities|Array|Get(acopy) (Class|RandomWalkLibrary|GetOutOfBoundsNeighbors (Utilities|Array|Get(acopy) _all_tile_coordinates (- (Variables|Default|GetCurrent%20Round) 1)) (Variables|WorldSettings|GetChunk%20Size)) (Default|GetRandomIntegerinRange (Variables|Default|GetRandom%20Noise%20Util) 0 (Utilities|Array|LastIndex _all_tile_coordinates))) (Utilities|Array|Get(acopy) (Variables|Default|GetAll%20Tile%20Coordinates) (+ (Variables|Default|GetCurrent%20Round) 1)))))))