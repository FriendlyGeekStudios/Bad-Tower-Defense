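; A single map tile in a chunked landscape that can hold a tower or become a road.
; Generate stretches its height by 2D noise and MPC_Landscape parameters, sets its type against a water-size threshold, and labels its local and global coordinates.
; Towers spawn at the mesh's MountPoint socket, and cursor hover applies an overlay highlight to tile and tower.
; Road conversion swaps material, resets height and sets the default nav area.
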(event Custom|OnBeginCursorOver_Event
  (params (TouchedActor :type Actor%20Object%20Reference))
  (CallFunction|EnableHighlight))

(event Custom|OnEndCursorOver_Event
  (params (TouchedActor :type Actor%20Object%20Reference))
  (CallFunction|DisableHighlight))

(event EventBeginPlay
  (Variables|/Script/Engine.PlayerController|SetbEnableMouseOverEvents (Game|GetPlayerController 0) true)
  (EventDispatchers|AssignOnBeginCursorOver (delegate Custom|OnBeginCursorOver_Event))
  (EventDispatchers|AssignOnEndCursorOver (delegate Custom|OnEndCursorOver_Event)))

(fn ConstructionScript
  (bind _asbp_chunk (Utilities|Casting|CastToBP_Chunk (Components|GetOwner (Variables|Default|GetDefaultSceneRoot)))
    (:then
      (Variables|Default|SetRandom%20Noise%20Util (Variables|/Game/Blueprints/Map/BP_Chunk.BP_Chunk_C|GetRandom%20Noise%20Util _asbp_chunk)))
    (:CastFailed
      (bind _returnvalue (Actor|GetActorOfClass "/Game/Blueprints/BP_RandomWrapper.BP_RandomWrapper_C"))
      (Variables|Default|SetRandom%20Noise%20Util _returnvalue))))

(fn Generate
  (params (Coordinate%20X :type Integer) (Coordinate%20Y :type Integer))
  (bind _coordinates (CallFunction|GetGlobalCoordinates))
  (bind _tile (Variables|Default|GetTile))
  (bind _label (Variables|Default|GetLabel))
  (bind _returnvalue (Transformation|GetWorldLocation _tile))
  (Variables|Default|SetCoordinate%20X Coordinate%20X)
  (Variables|Default|SetCoordinate%20Y Coordinate%20Y)
  (bind _asbp_chunk (Utilities|Casting|CastToBP_Chunk (Actor|GetParentActor)))
  (Variables|Default|SetParent%20Chunk _asbp_chunk)
  (bind _returnvalue_2 (Rendering|Material|GetScalarParameterValue "/Game/Materials/MPC_Landscape.MPC_Landscape" "Node Height Multiplier" :!class /Script/Engine.KismetMaterialLibrary))
  (Transformation|SetRelativeScale3D (Variables|Default|GetTile) (+ (Variables|/Script/Engine.SceneComponent|GetRelativeScale3D (Variables|Default|GetTile)) (Math|Vector|MakeVector 0.0 0.0 (* (Math|Float|Absolute(Float) (Default|GetNoise2D (Variables|Default|GetRandom%20Noise%20Util) (.x _returnvalue) (.y _returnvalue))) _returnvalue_2))))
  (bind _returnvalue_3 (Rendering|Material|GetScalarParameterValue "/Game/Materials/MPC_Landscape.MPC_Landscape" "Water Size" :!class /Script/Engine.KismetMaterialLibrary))
  (bind _returnvalue_4 (Rendering|Material|GetScalarParameterValue "/Game/Materials/MPC_Landscape.MPC_Landscape" "Node Height Multiplier" :!class /Script/Engine.KismetMaterialLibrary))
  (if (> (.z (Variables|/Script/Engine.SceneComponent|GetRelativeScale3D (Variables|Default|GetTile))) (/ _returnvalue_4 _returnvalue_3))
    (Variables|Default|SetTile%20Type "NewEnumerator2")
    (else
      (Variables|Default|SetTile%20Type "NewEnumerator0")))
  (bind _asbp_chunk_2 (Utilities|Casting|CastToBP_Chunk (Actor|GetParentActor)))
  (Rendering|Components|TextRender|SetText _label (Utilities|Text|FormatText "({X},{Y}) [({Global X}, {Global Y})]" (Variables|Default|GetCoordinate%20X) (Variables|Default|GetCoordinate%20Y) (.x _coordinates) (.y _coordinates)))
  (Transformation|SetWorldLocation _label (Transformation|GetSocketLocation (Variables|Default|GetTile) "MountPoint") false false))

(fn CreateTower
  (params (Tower%20Type :type BP%20Tower%20Base%20Class%20Reference))
  (bind _returnvalue (Game|SpawnActorfromClass Tower%20Type (Math|Transform|MakeTransform (Transformation|GetSocketLocation (Variables|Default|GetTile) "MountPoint") "0, 0, 0" "1.000000,1.000000,1.000000") "AdjustIfPossibleButAlwaysSpawn" "MultiplyWithRoot" self 0))
  (Variables|Default|SetTower _returnvalue))

(fn DestroyTower
  (bind _tower (Variables|Default|GetTower))
  (Utilities|IsValid _tower
    (:Is%20Valid
      (Actor|DestroyActor _tower))))

(fn EnableHighlight
  (bind _tower (Variables|Default|GetTower))
  (bind _highlight_material (Variables|Default|GetHighlight%20Material))
  (Rendering|Material|SetOverlayMaterial (Variables|Default|GetTile) _highlight_material :!class /Script/Engine.MeshComponent)
  (Utilities|IsValid _tower
    (:Is%20Valid
      (Rendering|Material|SetOverlayMaterial (Variables|/Game/Blueprints/Towers/BP_TowerBase.BP_TowerBase_C|GetTower _tower) _highlight_material :!class /Script/Engine.MeshComponent))))

(fn DisableHighlight
  (bind _tower (Variables|Default|GetTower))
  (Rendering|Material|SetOverlayMaterial (Variables|Default|GetTile) 0 :!class /Script/Engine.MeshComponent)
  (Utilities|IsValid _tower
    (:Is%20Valid
      (Rendering|Material|SetOverlayMaterial (Variables|/Game/Blueprints/Towers/BP_TowerBase.BP_TowerBase_C|GetTower _tower) 0 :!class /Script/Engine.MeshComponent))))

(fn GetGlobalCoordinates
  (bind _parent_chunk (Variables|Default|GetParent%20Chunk))
  (bind _chunkheight (Variables|/Game/Blueprints/Map/BP_Chunk.BP_Chunk_C|GetChunkHeight _parent_chunk))
  (return (Utilities|Struct|MakeCoordinate2D (+ (* (Variables|/Game/Blueprints/Map/BP_Chunk.BP_Chunk_C|GetCoordinate%20X _parent_chunk) _chunkheight) (Variables|Default|GetCoordinate%20X)) (+ (* _chunkheight (Variables|/Game/Blueprints/Map/BP_Chunk.BP_Chunk_C|GetCoordinate%20Y _parent_chunk)) (Variables|Default|GetCoordinate%20Y)))))

(fn UpdateMaterial
  (params (New%20Material :type Material%20Instance%20Object%20Reference))
  (Rendering|Material|SetMaterial (Variables|Default|GetTile) 0 New%20Material))

(fn ConverttoRoadTile
  (bind _tile (Variables|Default|GetTile))
  (bind _relativescale3d (Variables|/Script/Engine.SceneComponent|GetRelativeScale3D _tile))
  (Variables|Default|SetTile%20Type "NewEnumerator3")
  (Rendering|Material|SetMaterial (Variables|Default|GetTile) 0 "/Game/Materials/M_Road.M_Road")
  (Class|NavModifierComponent|SetAreaClass (Variables|Default|GetNavModifier) "/Script/NavigationSystem.NavArea_Default")
  (bind _returnvalue (Rendering|Material|GetScalarParameterValue "/Game/Materials/MPC_Landscape.MPC_Landscape" "Node Height Multiplier" :!class /Script/Engine.KismetMaterialLibrary))
  (Transformation|SetRelativeScale3D _tile (Math|Vector|MakeVector (.x _relativescale3d) (.y _relativescale3d) (* 0.3 _returnvalue))))